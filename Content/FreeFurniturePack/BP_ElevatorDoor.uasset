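; Elevator door Blueprint that opens and closes two sliding panels and handles the start and end of a delivery run.
; A timeline lerps both panels, opening them six seconds after BeginPlay and reversing to close.
; The intro box closes the doors and starts delivery via BP_GameManager once, or reopens them once when FinishFlag is set.
; With that flag set, the Victory overlap shows the win widget, disables player control and plays a completion sound.
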(event OnComponentBeginOverlap(introCloseBox)
  (params (OverlappedComponent :type Primitive%20Component%20Object%20Reference) (OtherActor :type Actor%20Object%20Reference) (OtherComp :type Primitive%20Component%20Object%20Reference) (OtherBodyIndex :type Integer) (bFromSweep :type Boolean) (SweepResult :type Hit%20Result%20Structure%20%28by%20ref%29))
  (Utilities|Casting|CastToBP_ThirdPersonCharacter OtherActor)
  (if (Variables|Default|GetfinishFlag)
    (Utilities|FlowControl|DoOnce false
      (:Completed
        (CallFunction|OpenAnimation)))
    (else
      (Utilities|FlowControl|DoOnce false
        (:Completed
          (bind _returnvalue (Actor|GetActorOfClass "/Game/Blueprints/Apartment/BP_GameManager.BP_GameManager_C"))
          (Default|StartDelivery _returnvalue)
          (CallFunction|CloseAnimation))))))

(event OnComponentBeginOverlap(victory)
  (params (OverlappedComponent :type Primitive%20Component%20Object%20Reference) (OtherActor :type Actor%20Object%20Reference) (OtherComp :type Primitive%20Component%20Object%20Reference) (OtherBodyIndex :type Integer) (bFromSweep :type Boolean) (SweepResult :type Hit%20Result%20Structure%20%28by%20ref%29))
  (bind _returnvalue (Game|GetPlayerController 0))
  (bind _returnvalue_2 (Game|GetPlayerController 0))
  (Utilities|Casting|CastToBP_ThirdPersonCharacter OtherActor)
  (if (Variables|Default|GetfinishFlag)
    (Development|PrintString "victory!" true true "(R=0.000000,G=0.660000,B=1.000000,A=1.000000)" 1e+01)
    (bind _returnvalue_3 (UserInterface|CreateWidget "/Game/WidgetsUI/W_Win.W_Win_C"))
    (UserInterface|Viewport|AddtoViewport _returnvalue_3 0)
    (Input|SetInputModeUIOnly _returnvalue_2 _returnvalue_3 "DoNotLock" false)
    (Variables|/Script/Engine.PlayerController|SetbShowMouseCursor _returnvalue_2 true)
    (bind _asbp_third_person_character (Utilities|Casting|CastToBP_ThirdPersonCharacter (Game|GetPlayerCharacter 0)))
    (Pawn|Components|CharacterMovement|DisableMovement (Variables|/Script/Engine.Character|GetCharacterMovement _asbp_third_person_character))
    (Input|SetIgnoreLookInput _returnvalue true)
    (Input|SetIgnoreMoveInput _returnvalue true)
    (Class|FMODBlueprintStatics|PlayEvent2D "/Game/FMOD/Events/MUS/Day_Completed.Day_Completed")))

(event Custom|OpenAnimation
  (bind _alpha (Timeline|OpenTimeline PlayFromStart)
    (:Update
      (Transformation|SetRelativeLocation (Variables|Default|GetL_Door) (Math|Vector|Lerp(Vector) (Variables|Default|GetL_Door_ClosePos) (Variables|Default|GetL_DoorOpenPos) _alpha) false false)
      (Transformation|SetRelativeLocation (Variables|Default|GetR_Door) (Math|Vector|Lerp(Vector) (Variables|Default|GetR_Door_ClosePos) (Variables|Default|GetR_DoorOpenPos) _alpha) false false))))

(event Custom|CloseAnimation
  (bind _alpha (Timeline|OpenTimeline ReverseFromEnd)
    (:Update
      (Transformation|SetRelativeLocation (Variables|Default|GetL_Door) (Math|Vector|Lerp(Vector) (Variables|Default|GetL_Door_ClosePos) (Variables|Default|GetL_DoorOpenPos) _alpha) false false)
      (Transformation|SetRelativeLocation (Variables|Default|GetR_Door) (Math|Vector|Lerp(Vector) (Variables|Default|GetR_Door_ClosePos) (Variables|Default|GetR_DoorOpenPos) _alpha) false false))))

(event EventBeginPlay
  (Variables|Default|SetR_Door_ClosePos (Variables|/Script/Engine.SceneComponent|GetRelativeLocation (Variables|Default|GetR_Door)))
  (Variables|Default|SetR_DoorOpenPos (Math|Vector|MakeVector -72.0 (.y (Variables|Default|GetR_Door_ClosePos)) (.z (Variables|Default|GetR_Door_ClosePos))))
  (Variables|Default|SetL_Door_ClosePos (Variables|/Script/Engine.SceneComponent|GetRelativeLocation (Variables|Default|GetL_Door)))
  (Variables|Default|SetL_DoorOpenPos (Math|Vector|MakeVector 72.0 (.y (Variables|Default|GetL_Door_ClosePos)) (.z (Variables|Default|GetL_Door_ClosePos))))
  (Utilities|FlowControl|Delay 6.0)
  (CallFunction|OpenAnimation))

(fn ConstructionScript)