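; BP_ElevatorLight is a rect light Blueprint, named for an elevator, that flickers continuously.
; From BeginPlay, SetFlickerTarget re-calls itself after a short random delay, picking a new random low intensity target each cycle.
; Tick eases the light's intensity toward that target with FInterpTo, smoothing the flicker.
; An unconnected branch that sets intensity directly never runs.
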(event Custom|SetFlickerTarget
  (Utilities|FlowControl|Delay (Math|Random|RandomFloatinRange 0.02 0.4))
  (Variables|Default|SetflickerTarget (Math|Random|RandomFloatinRange 0.07 0.2))
  (CallFunction|SetFlickerTarget))

(event EventBeginPlay
  (CallFunction|SetFlickerTarget))

(event EventTick
  (params (DeltaSeconds :type Float%20%28single-precision%29))
  (Rendering|Components|Light|SetIntensity (Variables|Default|GetRectLight) (Math|Interpolation|FInterpTo (Variables|/Script/Engine.LightComponentBase|GetIntensity (Variables|Default|GetRectLight)) (Variables|Default|GetflickerTarget) DeltaSeconds 1e+01)))

(fn ConstructionScript)