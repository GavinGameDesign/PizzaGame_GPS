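; BP_Hideables is an interactable hiding spot that toggles whether the player character is hiding.
; Its Interact event finds BP_ThirdPersonCharacter with GetActorOfClass and uses a FlipFlop to alternate IsHiding between true and false.
; The HideBox overlap events are empty, and leftover overlap-style logic for setting IsHiding on the player pawn is disconnected.
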(event OnComponentBeginOverlap(HideBox)
  (params (OverlappedComponent :type Primitive%20Component%20Object%20Reference) (OtherActor :type Actor%20Object%20Reference) (OtherComp :type Primitive%20Component%20Object%20Reference) (OtherBodyIndex :type Integer) (bFromSweep :type Boolean) (SweepResult :type Hit%20Result%20Structure%20%28by%20ref%29)))

(event OnComponentEndOverlap(HideBox)
  (params (OverlappedComponent :type Primitive%20Component%20Object%20Reference) (OtherActor :type Actor%20Object%20Reference) (OtherComp :type Primitive%20Component%20Object%20Reference) (OtherBodyIndex :type Integer)))

(event EventInteract
  ;[0.001816 0 0.7219] Set Player Hiding Or Not Hiding On Interact
  (bind _returnvalue (Actor|GetActorOfClass "/Game/ThirdPerson/Blueprints/BP_ThirdPersonCharacter.BP_ThirdPersonCharacter_C"))
  (Utilities|FlowControl|FlipFlop
    (:A
      (Variables|/Game/ThirdPerson/Blueprints/BP_ThirdPersonCharacter.BP_ThirdPersonCharacter_C|SetisHiding _returnvalue true))
    (:B
      (Variables|/Game/ThirdPerson/Blueprints/BP_ThirdPersonCharacter.BP_ThirdPersonCharacter_C|SetisHiding _returnvalue false))))

(fn ConstructionScript)