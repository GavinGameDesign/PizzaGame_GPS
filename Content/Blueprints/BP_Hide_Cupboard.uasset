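; BP_Hide_Cupboard is an interactable double-door cupboard, named as a hiding spot, that toggles its doors on interaction.
; Interact runs the parent logic, then AnimateDoor, where a FlipFlop alternates between playing DoorOpenTimeline from start and reversing it from end.
; The timeline alpha swings Door and Door1 in opposite directions through mirrored rotation lerps.
; AnimateDoor sets the timeline play rate to zero before each toggle.
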(event Custom|AnimateDoor
  (Components|Timeline|SetPlayRate (Variables|Default|GetDoorOpenTimeline) 0.0)
  (Utilities|FlowControl|FlipFlop
    (:A
      (bind _alpha (Timeline|DoorOpenTimeline PlayFromStart)
        (:Update
          (Transformation|SetRelativeRotation (Variables|Default|GetDoor) (Math|Rotator|Lerp(Rotator) "0, 0, 0" "0.000000,100.000000,0.000000" _alpha) false false)
          (Transformation|SetRelativeRotation (Variables|Default|GetDoor1) (Math|Rotator|Lerp(Rotator) "0, 0, 0" "0.000000,-100.000000,0.000000" _alpha) false false))))
    (:B
      (Timeline|DoorOpenTimeline ReverseFromEnd))))

(event EventInteract
  (|CallParentFunction)
  (CallFunction|AnimateDoor))

(fn ConstructionScript
  (|CallParentFunction))