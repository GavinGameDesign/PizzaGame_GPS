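; Game manager that runs the apartment pizza-delivery loop, from randomized orders to the exit objective.
; At start it shuffles floor shapes and builds random standard and additional deliveries, though only standard ones get started.
; Each standard delivery's timer scales with distance, floor gap and killer count, updating WB_Delivery.
; Door deliveries freeze the player for NPC dialogue, while timeouts spawn seeking killers; finishing all deliveries flags the elevator.
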(event Custom|StartDelivery
  (bind _wb_delivery (Variables|References|GetWB_Delivery))
  ;[0.5344 0.5344 0.5344] Comment
  (bind _output_get (Variables|Default|SetcurrentDeliveryIndex 0))
  (switch Utilities|FlowControl|Switch|SwitchonE_DeliveryType (.deliveryType (Utilities|Struct|BreakF_Delivery (Utilities|Array|Get(acopy) (Variables|Default|GetdeliveryInstructions) _output_get)))
    (:NewEnumerator0
      (Variables|References|SetcurrentStandardDoorToDeliverTo (.doorActor (Utilities|Struct|BreakF_Delivery (Utilities|Array|Get(acopy) (Variables|Default|GetdeliveryInstructions) _output_get))))
      (bind _deliverytime (CallFunction|CalculateDeliveryTime (.doorActor (Utilities|Struct|BreakF_Delivery (Utilities|Array|Get(acopy) (Variables|Default|GetdeliveryInstructions) _output_get)))))
      (CallFunction|StartStandardDeliveryTimer (* _deliverytime (.deliveryTimeMultiplier (Utilities|Struct|BreakF_Delivery (Utilities|Array|Get(acopy) (Variables|Default|GetdeliveryInstructions) _output_get)))))
      (Default|UpdateDeliveryInstructions _wb_delivery (.floorShape (Utilities|Struct|BreakF_Delivery (Utilities|Array|Get(acopy) (Variables|Default|GetdeliveryInstructions) _output_get))) (.doorColor (Utilities|Struct|BreakF_Delivery (Utilities|Array|Get(acopy) (Variables|Default|GetdeliveryInstructions) _output_get))) (.doorNumber (Utilities|Struct|BreakF_Delivery (Utilities|Array|Get(acopy) (Variables|Default|GetdeliveryInstructions) _output_get))) false)
      (Default|SetDeliveryInstructionOpacity _wb_delivery false "Visible"))))

(event Custom|OngoingDeliveryTimer
  (bind _returnvalue (Utilities|Time|GetGameTimeinSeconds))
  (bind _standarddeliverystarttime (Variables|Default|GetstandardDeliveryStartTime))
  (bind _standarddeliverytimelimit (Variables|Default|GetstandardDeliveryTimeLimit))
  (bind _returnvalue_2 (- _returnvalue _standarddeliverystarttime))
  (bind _returnvalue_3 (- _standarddeliverytimelimit _returnvalue_2))
  ;[0.576 0.576 0.576] Standard Delivery Timer
  (if (>= _returnvalue_2 (Variables|Default|GetstandardDeliveryTimeLimit)) ; Is time limit over?
    (Default|TemporaryNoInterface (Variables|References|GetcurrentStandardDoorToDeliverTo))
    (CallFunction|FailedDelivery)
    (else
      (bind _output_get (Variables|Default|SetstandardDeliveryTimeLeft _returnvalue_3))
      (Default|UpdateDeliveryTimer (Variables|References|GetWB_Delivery) (Math|Conversions|ToFloat(Integer) (Math|Float|Round _returnvalue_3)))
      (Default|UpdatePizzaTimer (Variables|References|GetWB_Delivery) _output_get _standarddeliverytimelimit))))

(event Custom|StartStandardDeliveryTimer
  (params (timeLimit :type Float%20%28double-precision%29))
  ;[0.576 0.576 0.576] Standard Delivery Timer
  (Variables|Default|SetstandardDeliveryTimeLimit timeLimit)
  (Variables|Default|SetstandardDeliveryStartTime (Utilities|Time|GetGameTimeinSeconds))
  (bind _returnvalue (Utilities|Time|SetTimerbyEvent (delegate Custom|OngoingDeliveryTimer) 0.5 true)))

(event Custom|FailedDelivery
  ;[0.576 0.576 0.576] Standard Delivery Timer
  (Utilities|Time|ClearandInvalidateTimerbyHandle (stale Custom|StartStandardDeliveryTimer _returnvalue))
  (CallFunction|SpawnNewKiller)
  (Utilities|FlowControl|Delay 1.0)
  (CallFunction|NextDeliveryStart))

(event Custom|SucceedDelivery
  ;[0.576 0.576 0.576] Standard Delivery Timer
  (Utilities|Time|ClearandInvalidateTimerbyHandle (stale Custom|StartStandardDeliveryTimer _returnvalue)))

(event Custom|DeliveredToDoor
  (params (givenDoor :type BP%20Floor%20Door%20Object%20Reference))
  (bind _doorsnpc (Variables|/Game/Blueprints/Apartment/Door/BP_FloorDoor.BP_FloorDoor_C|GetdoorsNPC givenDoor))
  (bind _doorsnpc_2 (Variables|/Game/Blueprints/Apartment/Door/BP_FloorDoor.BP_FloorDoor_C|GetdoorsNPC givenDoor))
  (bind _returnvalue (Transformation|GetActorLocation _doorsnpc))
  (bind _returnvalue_2 (+ (.z _returnvalue) 1e+02))
  (bind _returnvalue_3 (Math|Vector|MakeVector (.x _returnvalue) (.y _returnvalue) _returnvalue_2))
  ;[0.5135 0.5135 0.5135 1 32] Door Delivery
  (Utilities|IsValid givenDoor
    (:Is%20Valid
      (CallFunction|FreezeUnfreezePlayer true)
      (Default|SpawnDoorNPC givenDoor)
      (if (or (== givenDoor (Variables|References|GetcurrentStandardDoorToDeliverTo)) (== givenDoor (Variables|References|GetcurrentAdditionalDoorToDeliverTo)))
        (Development|PrintString "CORRECT DOOR!" true true "(R=0.000000,G=0.787500,B=0.096352,A=1.000000)" 6.0)
        (CallFunction|SucceedDelivery)
        (if (<= (Variables|Default|GetstandardDeliveryTimeLeft) 5.0)
          (Utilities|FlowControl|Delay 1.0) ; Kncck Time
          (Default|SmoothCamLookat (Variables|References|GetPlayer) _returnvalue_3)
          (Default|Dialogue _doorsnpc_2 "NewEnumerator1")
          (else
            (Utilities|FlowControl|Delay 1.0) ; Kncck Time
            (Default|SmoothCamLookat (Variables|References|GetPlayer) _returnvalue_3)
            (Default|Dialogue _doorsnpc_2 "NewEnumerator0")))
        (else
          (Development|PrintString "WRONG DOOR :(" true true "(R=1.000000,G=0.553315,B=0.000000,A=1.000000)" 6.0)
          (Utilities|FlowControl|Delay 1.0) ; Kncck Time
          (Default|SmoothCamLookat (Variables|References|GetPlayer) _returnvalue_3)
          (Default|Dialogue _doorsnpc_2 "NewEnumerator8")))
      (if (Variables|/Game/Blueprints/BP_DialogueManagerJacob.BP_DialogueManagerJacob_C|GetdialogueRunning (Variables|References|GetDialogueManager)) :!label _label
        (Utilities|FlowControl|Delay 0.2)
        (goto _label)
        (else
          (Default|CloseDoor _doorsnpc_2)
          (Default|PlayAnimation givenDoor)
          (Default|SmoothCamLookatUndo (Variables|References|GetPlayer))
          (Utilities|FlowControl|Delay 1.0)
          (CallFunction|FreezeUnfreezePlayer false)
          (Actor|DestroyActor _doorsnpc_2)
          (CallFunction|NextDeliveryStart))))))

(event Custom|NextDeliveryStart
  (bind _wb_delivery (Variables|References|GetWB_Delivery))
  (bind _wb_delivery_2 (Variables|References|GetWB_Delivery))
  ;[0.5344 0.5344 0.5344] Comment
  (Math|Integer|IncrementInt (Variables|Default|GetcurrentDeliveryIndex)
    (:%20%20
      (if (> (Variables|Default|GetcurrentDeliveryIndex) (Variables|Default|GetdeliveryAmount)) ; Are your deliveries done?
        (Development|PrintString "You have finished all deliveries!" true true "(R=0.000000,G=1.000000,B=0.125820,A=1.000000)" 15.0)
        (Default|SetDeliveryInstructionOpacity _wb_delivery false "Hidden")
        (Default|ToggleExitText _wb_delivery "Visible")
        (Variables|/Game/WidgetsUI/WB_Delivery.WB_Delivery_C|SetobjectiveText (Variables|References|GetWB_Delivery) "Exit the building safely!")
        (Variables|/Game/FreeFurniturePack/BP_ElevatorDoor.BP_ElevatorDoor_C|SetfinishFlag (Variables|Default|GetElevator) true)
        (else
          (switch Utilities|FlowControl|Switch|SwitchonE_DeliveryType (.deliveryType (Utilities|Struct|BreakF_Delivery (Utilities|Array|Get(acopy) (Variables|Default|GetdeliveryInstructions) (stale Custom|StartDelivery _output_get))))
            (:NewEnumerator0
              (Variables|References|SetcurrentStandardDoorToDeliverTo (.doorActor (Utilities|Struct|BreakF_Delivery (Utilities|Array|Get(acopy) (Variables|Default|GetdeliveryInstructions) (stale Custom|StartDelivery _output_get)))))
              (bind _deliverytime (CallFunction|CalculateDeliveryTime (.doorActor (Utilities|Struct|BreakF_Delivery (Utilities|Array|Get(acopy) (Variables|Default|GetdeliveryInstructions) (stale Custom|StartDelivery _output_get))))))
              (CallFunction|StartStandardDeliveryTimer (* _deliverytime (.deliveryTimeMultiplier (Utilities|Struct|BreakF_Delivery (Utilities|Array|Get(acopy) (Variables|Default|GetdeliveryInstructions) (stale Custom|StartDelivery _output_get))))))
              (Default|UpdateDeliveryInstructions _wb_delivery_2 (.floorShape (Utilities|Struct|BreakF_Delivery (Utilities|Array|Get(acopy) (Variables|Default|GetdeliveryInstructions) (stale Custom|StartDelivery _output_get)))) (.doorColor (Utilities|Struct|BreakF_Delivery (Utilities|Array|Get(acopy) (Variables|Default|GetdeliveryInstructions) (stale Custom|StartDelivery _output_get)))) (.doorNumber (Utilities|Struct|BreakF_Delivery (Utilities|Array|Get(acopy) (Variables|Default|GetdeliveryInstructions) (stale Custom|StartDelivery _output_get)))) false)
              (Default|SetDeliveryInstructionOpacity _wb_delivery_2 false "Visible"))))))))

(event EventBeginPlay
  (Utilities|FlowControl|Sequence
    (:then_0
      (bind _asbp_third_person_character (Utilities|Casting|CastToBP_ThirdPersonCharacter (Pawn|GetControlledPawn (Game|GetPlayerController 0))))
      (Variables|References|SetPlayer _asbp_third_person_character))
    (:then_1
      (CallFunction|ShuffleFloorShapes)
      (CallFunction|GenerateDeliveryInstructions))
    (:then_2
      (Utilities|FlowControl|Delay 0.2)
      (bind _foundwidgets (Widget|GetAllWidgetsOfClass "/Game/WidgetsUI/WB_Delivery.WB_Delivery_C" true))
      (Variables|References|SetWB_Delivery (Utilities|Array|Get(acopy) _foundwidgets))
      (bind _returnvalue (Actor|GetActorOfClass "/Game/Blueprints/BP_DialogueManagerJacob.BP_DialogueManagerJacob_C"))
      (Variables|References|SetDialogueManager _returnvalue)
      (Variables|/Game/WidgetsUI/WB_Delivery.WB_Delivery_C|SetobjectiveText (Variables|References|GetWB_Delivery) "Deliver all the pizzas.")
      (bind _returnvalue_2 (Actor|GetActorOfClass "/Game/FreeFurniturePack/BP_ElevatorDoor.BP_ElevatorDoor_C"))
      (Variables|Default|SetElevator _returnvalue_2))))

(fn ConstructionScript)

(fn ShuffleFloorShapes
  (Utilities|Array|Shuffle (Variables|Default|GetpossibleShapes))
  (for (_array_element _array_index) (Variables|Default|GetfloorArray)
    (Variables|/Game/Blueprints/Apartment/BP_FloorClass.BP_FloorClass_C|SetfloorShape _array_element (Utilities|Enum|ByteToEnumE_ShapeTypes (Math|Conversions|ToByte(Integer) (Utilities|Array|Get(acopy) (Variables|Default|GetpossibleShapes) _array_index))))
    (Default|Start _array_element)))

(fn GenerateDeliveryInstructions
  (bind _deliveryinstructions (Variables|Default|GetdeliveryInstructions))
  ;[1 1 1] Generate Standard Deliveries
  (Utilities|FlowControl|ForLoopwithBreak 0 (- (Variables|Default|GetdeliveryAmount) 1)
    (:LoopBody
      (LocalVariables|SetfloorToInspect (.OutItem (Utilities|Array|Random (Variables|Default|GetfloorArray))))
      (LocalVariables|SetdoorToInspect (.OutItem (Utilities|Array|Random (Variables|/Game/Blueprints/Apartment/BP_FloorClass.BP_FloorClass_C|GetdoorsOnFloor (LocalVariables|GetfloorToInspect)))))
      (Utilities|Array|Add (Variables|Default|GetdeliveryInstructions) (Utilities|Struct|MakeF_Delivery "NewEnumerator0" (Utilities|Array|FindItem (Variables|Default|GetfloorArray) (LocalVariables|GetfloorToInspect)) (Variables|/Game/Blueprints/Apartment/BP_FloorClass.BP_FloorClass_C|GetfloorShape (LocalVariables|GetfloorToInspect)) (Variables|/Game/Blueprints/Apartment/Door/BP_FloorDoor.BP_FloorDoor_C|Getcolor (LocalVariables|GetdoorToInspect)) (Variables|/Game/Blueprints/Apartment/Door/BP_FloorDoor.BP_FloorDoor_C|Getnumber (LocalVariables|GetdoorToInspect)) 1.0 (LocalVariables|GetdoorToInspect))))
    (:Completed
      ;[1 1 1] Generate Additional Tasks
      (Utilities|FlowControl|ForLoopwithBreak 1 (Variables|Default|GetadditionalTasksAmount)
        (:LoopBody
          (LocalVariables|SetfloorToInspect (.OutItem (Utilities|Array|Random (Variables|Default|GetfloorArray))))
          (LocalVariables|SetdoorToInspect (.OutItem (Utilities|Array|Random (Variables|/Game/Blueprints/Apartment/BP_FloorClass.BP_FloorClass_C|GetdoorsOnFloor (LocalVariables|GetfloorToInspect)))))
          (bind _output_get (LocalVariables|SetadditionalIndexToInspect (Math|Random|RandomIntegerinRange 1 (Utilities|Array|LastIndex (Variables|Default|GetdeliveryInstructions))) :!label _label))
          (if (Utilities|Enum|Equal(Enum) (.deliveryType (Utilities|Struct|BreakF_Delivery (Utilities|Array|Get(acopy) (Variables|Default|GetdeliveryInstructions) _output_get))) "NewEnumerator0") ; Check chosen index
            (if (Utilities|Array|IsValidIndex _deliveryinstructions (+ _output_get 1))
              (if (Utilities|Enum|Equal(Enum) (.deliveryType (Utilities|Struct|BreakF_Delivery (Utilities|Array|Get(acopy) _deliveryinstructions (+ _output_get 1)))) "NewEnumerator0") ; Check index in front
                _
                (else
                  (goto _label))))
            (Utilities|Array|Insert (Variables|Default|GetdeliveryInstructions) (Utilities|Struct|MakeF_Delivery "NewEnumerator1" (Utilities|Array|FindItem (Variables|Default|GetfloorArray) (LocalVariables|GetfloorToInspect)) (Variables|/Game/Blueprints/Apartment/BP_FloorClass.BP_FloorClass_C|GetfloorShape (LocalVariables|GetfloorToInspect)) (Variables|/Game/Blueprints/Apartment/Door/BP_FloorDoor.BP_FloorDoor_C|Getcolor (LocalVariables|GetdoorToInspect)) (Variables|/Game/Blueprints/Apartment/Door/BP_FloorDoor.BP_FloorDoor_C|Getnumber (LocalVariables|GetdoorToInspect)) 1.0 (LocalVariables|GetdoorToInspect)) (LocalVariables|GetadditionalIndexToInspect)) ; Insert additional task but NOT after first task and NOT after an additional task.
            (else
              (goto _label))))
        (:Completed
          ;[1 1 1] Provide Additional Time when Additional Tasking
          (for (_array_element _array_index) (Variables|Default|GetdeliveryInstructions)
            (if (Utilities|Enum|Equal(Enum) (.deliveryType (Utilities|Struct|BreakF_Delivery _array_element)) "NewEnumerator1")
              (Utilities|Struct|SetmembersinF_Delivery _array_element 1.25)
              (Utilities|Struct|SetmembersinF_Delivery (Utilities|Array|Get(acopy) (Variables|Default|GetdeliveryInstructions) (LocalVariables|GetpreviousDeliveryIndex)) 1.5)
              (LocalVariables|SetpreviousDeliveryIndex _array_index)
              (else
                (LocalVariables|SetpreviousDeliveryIndex _array_index))))
          (return))))))

(fn CalculateDeliveryTime
  (params (floorDoor :type BP%20Floor%20Door%20Object%20Reference))
  (bind _returnvalue (Transformation|GetActorLocation floorDoor))
  (bind _player (Variables|References|GetPlayer))
  (bind _returnvalue_2 (Transformation|GetActorLocation _player))
  (return (Math|Float|Clamp(Float) (+ (* (/ (Math|Vector|Distance2D(Vector) _returnvalue _returnvalue_2) 6e+03) (LocalVariables|GetbaseTime)) (* (Math|Float|Floor (/ (Math|Float|Absolute(Float) (- (.Z (Math|Vector|BreakVector _returnvalue)) (.Z (Math|Vector|BreakVector _returnvalue_2)))) (LocalVariables|GetdistanceBetweenFloors))) (LocalVariables|GettimeToAddPerFloorDistance)) (* (Utilities|Array|Length (Variables|Default|GetkillerList)) (LocalVariables|GettimeToAddPerKiller))) 1e+01 1.8e+02)))

(fn FreezeUnfreezePlayer
  (params (isFreezePlayer :type Boolean))
  (bind _returnvalue (Game|GetPlayerController 0))
  (Input|SetIgnoreMoveInput _returnvalue isFreezePlayer)
  (Input|SetIgnoreLookInput _returnvalue isFreezePlayer)
  (Variables|/Game/ThirdPerson/Blueprints/BP_ThirdPersonCharacter.BP_ThirdPersonCharacter_C|SetdisableInteract (Variables|References|GetPlayer) isFreezePlayer))

(fn SpawnNewKiller
  (bind _currentstandarddoortodeliverto (Variables|References|GetcurrentStandardDoorToDeliverTo))
  (bind _actorseekspawnpoint (Variables|/Game/Blueprints/Apartment/Door/BP_FloorDoor.BP_FloorDoor_C|GetactorSeekSpawnPoint _currentstandarddoortodeliverto))
  (Variables|/Game/Blueprints/Apartment/Door/BP_FloorDoor.BP_FloorDoor_C|SetallowedToInterface _currentstandarddoortodeliverto false)
  (bind _returnvalue (Game|SpawnActorfromClass (Variables|/Game/Blueprints/Apartment/Door/BP_FloorDoor.BP_FloorDoor_C|GetnpcClass _currentstandarddoortodeliverto) (Math|Transform|MakeTransform (Transformation|GetWorldLocation _actorseekspawnpoint) (Transformation|GetWorldRotation _actorseekspawnpoint)) "Undefined" "MultiplyWithRoot" 0 0))
  (Utilities|Array|Add (Variables|Default|GetkillerList) _returnvalue)
  (Default|Dialogue _returnvalue "NewEnumerator2")
  (Default|BeginSeeking _returnvalue))