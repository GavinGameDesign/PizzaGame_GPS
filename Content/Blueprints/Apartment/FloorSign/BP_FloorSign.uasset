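; BP_FloorSign is an apartment floor sign that displays one of four shapes: circle, triangle, square or star.
; A switch on ShapeType sets the Shape component's material instance and a relative rotation suited to that shape, with circle and square sharing one rotation.
; The Construction Script applies this from the current ShapeType, and the ChangeSign event stores a new shape and repeats the same switch, duplicated rather than shared.
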(event Custom|ChangeSign
  (params (shape :type E_ShapeTypes%20Enum :default "NewEnumerator0"))
  (Variables|Default|SetshapeType shape)
  (switch Utilities|FlowControl|Switch|SwitchonE_ShapeTypes (Variables|Default|GetshapeType)
    (:NewEnumerator0
      (Rendering|Material|SetMaterial (Variables|Default|GetShape) 0 "/Game/Blueprints/Apartment/FloorSign/Materials/MI_FloorSign_Circle.MI_FloorSign_Circle")
      (Transformation|SetRelativeRotation (Variables|Default|GetShape) "0.000000,180.000000,0.000000" false false :!label _label))
    (:NewEnumerator1
      (Rendering|Material|SetMaterial (Variables|Default|GetShape) 0 "/Game/Blueprints/Apartment/FloorSign/Materials/MI_FloorSign_Triangle.MI_FloorSign_Triangle")
      (Transformation|SetRelativeRotation (Variables|Default|GetShape) "0.000000,270.000000,0.000000" false false))
    (:NewEnumerator2
      (Rendering|Material|SetMaterial (Variables|Default|GetShape) 0 "/Game/Blueprints/Apartment/FloorSign/Materials/MI_FloorSign_Square.MI_FloorSign_Square")
      (goto _label))
    (:NewEnumerator3
      (Rendering|Material|SetMaterial (Variables|Default|GetShape) 0 "/Game/Blueprints/Apartment/FloorSign/Materials/MI_FloorSign_Star.MI_FloorSign_Star")
      (Transformation|SetRelativeRotation (Variables|Default|GetShape) "0.000000,198.000000,0.000000" false false))))

(fn ConstructionScript
  (switch Utilities|FlowControl|Switch|SwitchonE_ShapeTypes (Variables|Default|GetshapeType)
    (:NewEnumerator0
      (Rendering|Material|SetMaterial (Variables|Default|GetShape) 0 "/Game/Blueprints/Apartment/FloorSign/Materials/MI_FloorSign_Circle.MI_FloorSign_Circle")
      (Transformation|SetRelativeRotation (Variables|Default|GetShape) "0.000000,180.000000,0.000000" false false :!label _label))
    (:NewEnumerator1
      (Rendering|Material|SetMaterial (Variables|Default|GetShape) 0 "/Game/Blueprints/Apartment/FloorSign/Materials/MI_FloorSign_Triangle.MI_FloorSign_Triangle")
      (Transformation|SetRelativeRotation (Variables|Default|GetShape) "0.000000,270.000000,0.000000" false false))
    (:NewEnumerator2
      (Rendering|Material|SetMaterial (Variables|Default|GetShape) 0 "/Game/Blueprints/Apartment/FloorSign/Materials/MI_FloorSign_Square.MI_FloorSign_Square")
      (goto _label))
    (:NewEnumerator3
      (Rendering|Material|SetMaterial (Variables|Default|GetShape) 0 "/Game/Blueprints/Apartment/FloorSign/Materials/MI_FloorSign_Star.MI_FloorSign_Star")
      (Transformation|SetRelativeRotation (Variables|Default|GetShape) "0.000000,198.000000,0.000000" false false))))