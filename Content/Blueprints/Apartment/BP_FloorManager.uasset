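; BP_FloorManager randomizes which shape each apartment floor gets when play begins.
; It shuffles PossibleShapes, then pairs it by index with FloorArray, so each floor takes a different entry from the list.
; Each entry is converted through a byte to an E_ShapeTypes value, set as that floor's FloorShape, and followed by a Start call on the floor.
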(event EventBeginPlay
  (CallFunction|ShuffleFloorShapes))

(fn ConstructionScript)

(fn ShuffleFloorShapes
  (Utilities|Array|Shuffle (Variables|Default|GetpossibleShapes))
  (for (_array_element _array_index) (Variables|Default|GetfloorArray)
    (Variables|/Game/Blueprints/Apartment/BP_FloorClass.BP_FloorClass_C|SetfloorShape _array_element (Utilities|Enum|ByteToEnumE_ShapeTypes (Math|Conversions|ToByte(Integer) (Utilities|Array|Get(acopy) (Variables|Default|GetpossibleShapes) _array_index))))
    (Default|Start _array_element)))