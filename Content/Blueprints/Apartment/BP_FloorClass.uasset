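; BP_FloorClass represents an apartment floor with a number and shape, and sets up the doors on it.
; Its Start event prints the floor's identity, then runs door setup, or prints an error if the door list is empty.
; Setup draws a unique random two-digit-or-less number for each door, then assigns it and randomizes that door's color.
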(event Custom|Start
  (Development|PrintString (Utilities|String|Append "I am floor " (Utilities|String|ToString(Integer) (Variables|Default|GetfloorNumber)) " and my shape is " (Utilities|String|EnumtoString (Variables|Default|GetfloorShape))) true true "(R=0.000000,G=0.660000,B=1.000000,A=1.000000)" 1e+01)
  (if (!= (Utilities|Array|Length (Variables|Default|GetdoorsOnFloor)) 0)
    (CallFunction|GenerateDoorNumbers)
    (CallFunction|AssignDoorNumbersandColors)
    (else
      (Development|PrintString (Utilities|String|Append "ERROR: doorsOnFloor on " (Utilities|GetDisplayName self) " is empty!") true true "(R=1.000000,G=0.006474,B=0.000000,A=1.000000)" 2e+01))))

(fn ConstructionScript)

(fn GenerateDoorNumbers
  (while (not (LocalVariables|GetdoorsGenerated))
    (Utilities|Array|AddUnique (Variables|Default|GetdoorNumbers) (Math|Random|RandomIntegerinRange 1 99))
    (if (== (Utilities|Array|Length (Variables|Default|GetdoorNumbers)) (Utilities|Array|Length (Variables|Default|GetdoorsOnFloor)))
      (LocalVariables|SetdoorsGenerated true))))

(fn AssignDoorNumbersandColors
  (for (_array_element _array_index) (Variables|Default|GetdoorsOnFloor)
    (Default|SetDoorNumber _array_element (Utilities|Text|ToText(Integer) (Utilities|Array|Get(acopy) (Variables|Default|GetdoorNumbers) _array_index)))
    (Default|RandomizeDoorColor _array_element)))