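; BP_FloorDoor is an apartment door that serves as a delivery target, reporting to BP_GameManager with a knock sound when interacted with.
; Its number displays either plainly or as a random addition or subtraction puzzle, and a shared dynamic material tints door and frame.
; It spawns a randomly chosen NPC class inside, then swings open.
; A FlipFlop alternates timeline-driven opening and closing with sounds, and interaction can be briefly disabled.
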(event Custom|PlayAnimation
  (Utilities|FlowControl|FlipFlop
    (:A
      (Class|FMODBlueprintStatics|PlayEventatLocation "/Game/FMOD/Events/FOL/door_open.door_open" (Transformation|GetActorTransform))
      (bind _doorzrotation (Timeline|Open/Close_Door_Timeline PlayFromStart)
        (:Update
          (Transformation|SetRelativeRotation (Variables|Default|GetDoorMesh) (Math|Rotator|MakeRotator 0.0 0.0 (* _doorzrotation (Variables|Default|GetdoorOpenAmount))) false false))))
    (:B
      (Utilities|Time|SetTimerbyEvent (delegate Custom|CloseSound) 0.5)
      (Timeline|Open/Close_Door_Timeline ReverseFromEnd))))

(event Custom|SetDoorNumber
  (params (givenNumber :type Integer))
  (bind _output_get (Variables|Default|Setnumber givenNumber))
  (if (Math|Random|RandomBoolwithWeight 0.5)
    (Rendering|Components|TextRender|SetText (Variables|Default|GetdoorNumber) (Utilities|Text|ToText(Integer) _output_get))
    (elif (Math|Random|RandomBoolwithWeight 0.5)
      (Variables|Default|SetintDoorEvaluate (Math|Random|RandomIntegerinRange 0 (Variables|Default|Getnumber)))
      (Rendering|Components|TextRender|SetText (Variables|Default|GetdoorNumber) (Utilities|Text|ToText(String) (Utilities|String|Append (Utilities|String|ToString(Integer) (Variables|Default|GetintDoorEvaluate)) " + " (Utilities|String|ToString(Integer) (- (Variables|Default|Getnumber) (Variables|Default|GetintDoorEvaluate))))))
      (else
        (Variables|Default|SetintDoorEvaluate (Math|Random|RandomIntegerinRange (Variables|Default|Getnumber) (* (Variables|Default|Getnumber) 2)))
        (Rendering|Components|TextRender|SetText (Variables|Default|GetdoorNumber) (Utilities|Text|ToText(String) (Utilities|String|Append (Utilities|String|ToString(Integer) (Variables|Default|GetintDoorEvaluate)) " - " (Utilities|String|ToString(Integer) (- (Variables|Default|GetintDoorEvaluate) (Variables|Default|Getnumber))))))))))

(event Custom|RandomizeDoorColor
  (bind _output_get (Variables|Default|Setcolor (.OutItem (Utilities|Array|Random (Variables|Default|GetpossibleColors)))))
  (Rendering|Material|SetVectorParameterValue (Variables|Default|GetdoorMaterial) "DoorColor" (Math|Conversions|ToLinearColor(Color) _output_get) :!class /Script/Engine.MaterialInstanceDynamic))

(event Custom|SpawnDoorNPC
  (bind _actorinsidespawnpoint (Variables|Default|GetactorInsideSpawnPoint))
  (bind _returnvalue (Game|SpawnActorfromClass (Variables|Default|GetnpcClass) (Math|Transform|MakeTransform (Transformation|GetWorldLocation _actorinsidespawnpoint) (Transformation|GetWorldRotation _actorinsidespawnpoint)) "Undefined" "MultiplyWithRoot" 0 0))
  (bind _output_get (Variables|Default|SetdoorsNPC _returnvalue))
  (Utilities|FlowControl|Delay 1.0) ; Knock Time
  (Default|OpenDoor _output_get)
  (CallFunction|PlayAnimation))

(event Custom|TemporaryNoInterface
  (Variables|Default|SetallowedToInterface false)
  (Utilities|FlowControl|Delay 2.0)
  (Variables|Default|SetallowedToInterface true))

(event Custom|CloseSound
  (Class|FMODBlueprintStatics|PlayEventatLocation "/Game/FMOD/Events/FOL/door_close.door_close" (Transformation|GetActorTransform)))

(event EventInteract
  (if (Variables|Default|GetallowedToInterface)
    (Default|DeliveredtoDoor (Variables|Default|GetGameManager) self)
    (Audio|PlaySoundatLocation (Variables|Default|GetknockSound) (Transformation|GetActorLocation) "0, 0, 0" 1.0 1.0 0.0 0 0 0 0)))

(event EventBeginPlay
  (bind _returnvalue (Actor|GetActorOfClass "/Game/Blueprints/Apartment/BP_GameManager.BP_GameManager_C"))
  (Variables|Default|SetGameManager _returnvalue)
  (Variables|Default|SetnpcClass (.OutItem (Utilities|Array|Random (Variables|Default|GetpossbleNpcTypes)))))

(fn ConstructionScript
  (bind _returnvalue (Rendering|Material|CreateDynamicMaterialInstance (Variables|Default|GetDoorMesh) 0 "/Game/Blueprints/Apartment/Door/M_Door.M_Door" "None" :!class /Script/Engine.PrimitiveComponent))
  (bind _output_get (Variables|Default|SetdoorMaterial _returnvalue))
  (Rendering|Material|SetVectorParameterValue _output_get "DoorColor" (Math|Conversions|ToLinearColor(Color) (Variables|Default|Getcolor)) :!class /Script/Engine.MaterialInstanceDynamic)
  (Rendering|Material|SetMaterial (Variables|Default|GetDoorFrameMesh) 0 (Variables|Default|GetdoorMaterial)))